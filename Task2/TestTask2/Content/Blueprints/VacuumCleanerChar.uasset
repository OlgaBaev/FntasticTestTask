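; Vacuum cleaner character that starts moving when a referenced door fires its open event, travelling between a target actor and a source actor.
; A looping timer runs MoveModeChange, cycling forward, stop and backward phases with separate durations and skipping non-positive ones.
; Tick issues AIMoveTo for the current phase and plays a sound at the cleaner.
; Near either destination in XY, it switches to silence and disables movement, with no re-enable here.
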(event Custom|OpenDoor
  (Variables|Default|SetStartMovement true))

(event Custom|OpenTheD
  (CallFunction|OpenDoor))

(event EventBeginPlay
  (EventDispatchers|BindEventtoOpentheDoor (Variables|Default|GetOpenDoorRef) (delegate Custom|OpenTheD))
  (Variables|/Script/Engine.CharacterMovementComponent|SetMaxWalkSpeed (Variables|Character|GetCharacterMovement) 1e+02)
  (bind _output_get (Variables|Default|SetTime (Variables|Timers|GetTimeForward)))
  (Variables|Default|SetTimeLeft _output_get)
  (Utilities|Time|SetTimerbyFunctionName 0 "MoveModeChange" (Variables|Timers|GetMinTimeStep) true))

(event EventTick
  (params (DeltaSeconds :type Float%20%28single-precision%29))
  (bind _cleaner (Variables|Default|GetCleaner))
  (bind _returnvalue (Transformation|GetWorldLocation _cleaner))
  (if (Variables|Default|GetStartMovement)
    (if (>= (Variables|Default|GetMoveMode) 1)
      (Variables|Default|SetDestination (Variables|Default|GetTarget%20Actor))
      (AI|AIMoveTo self "0, 0, 0" (Variables|Default|GetDestination) 5.0 false :!label _label
        (:then
          (Audio|PlaySoundatLocation (Variables|Default|GetSound) (Transformation|GetWorldLocation (Variables|Default|GetCleaner)) "0, 0, 0" 1.0 1.0 0.0 0 0 0)
          (if (<= (Math|Float|Absolute(Float) (+ (* (- (.y _returnvalue) (.y (Transformation|GetActorLocation (Variables|Default|GetDestination)))) (- (.y _returnvalue) (.y (Transformation|GetActorLocation (Variables|Default|GetDestination))))) (* (- (.x _returnvalue) (.x (Transformation|GetActorLocation (Variables|Default|GetDestination)))) (- (.x _returnvalue) (.x (Transformation|GetActorLocation (Variables|Default|GetDestination))))))) 1.5e+02)
            (Variables|Default|SetSound "/Game/Audio/Silence.Silence")
            (Pawn|Components|CharacterMovement|DisableMovement (Variables|Character|GetCharacterMovement)))))
      (elif (<= (Variables|Default|GetMoveMode) -1)
        (Variables|Default|SetDestination (Variables|Default|GetSourceActor))
        (goto _label)
        (else
          (Class|NavMovementComponent|StopActiveMovement (Variables|Character|GetCharacterMovement)))))))

(fn ConstructionScript)

(fn MoveModeChange
  (if (>= (Variables|Default|GetTimeLeft) 0.1)
    (Variables|Default|SetTimeLeft (- (Variables|Default|GetTimeLeft) (Variables|Timers|GetMinTimeStep)))
    (else
      (if (>= (Variables|Default|GetMoveMode) 1) :!label _label
        (Variables|Default|SetTime (Variables|Timers|GetTimeStop))
        (Math|Integer|DecrementInt (Variables|Default|GetMoveMode) :!label _label_2
          (:%20%20
            _))
        (elif (>= (Variables|Default|GetMoveMode) 0)
          (Variables|Default|SetTime (Variables|Timers|GetTimeBackward))
          (goto _label_2)
          (else
            (Variables|Default|SetTime (Variables|Timers|GetTimeForward))
            (Variables|Default|SetMoveMode 1))))
      (bind _output_get (Variables|Default|SetTimeLeft (Variables|Default|GetTime)))
      (if (<= _output_get 0.0)
        (goto _label)))))