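; UseKey is an interactable door that rises when the player releases E near it.
; Box overlap begin and end enable and disable input, without checking which actor overlaps.
; E plays a timeline whose Open track drives an additive upward offset on Door each update.
; The same update chain runs through a short Delay to play the start-move sound at Door's relative location and call OpenTheDoor, so both can repeat during playback.
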(event OnComponentBeginOverlap(Box)
  (params (OverlappedComponent :type Primitive%20Component%20Object%20Reference) (OtherActor :type Actor%20Object%20Reference) (OtherComp :type Primitive%20Component%20Object%20Reference) (OtherBodyIndex :type Integer) (bFromSweep :type Boolean) (SweepResult :type Hit%20Result%20Structure%20%28by%20ref%29))
  (Input|EnableInput (Game|GetPlayerController 0)))

(event OnComponentEndOverlap(Box)
  (params (OverlappedComponent :type Primitive%20Component%20Object%20Reference) (OtherActor :type Actor%20Object%20Reference) (OtherComp :type Primitive%20Component%20Object%20Reference) (OtherBodyIndex :type Integer))
  (Input|DisableInput (Game|GetPlayerController 0)))

(event Input|KeyboardEvents|E
  (params (Key :type Key%20Structure :default "None"))
  (:Released
    (bind _open (Timeline|Timeline_0 Play)
      (:Update
        (Transformation|AddRelativeLocation (Variables|Default|GetDoor) (Math|Vector|MakeVector 0.0 0.0 (* _open 2.0)) false false)
        (Utilities|FlowControl|Delay 0.5)
        (Audio|PlaySoundatLocation (Variables|Default|GetStartMoveSound) (Variables|/Script/Engine.SceneComponent|GetRelativeLocation (Variables|Default|GetDoor)) "0, 0, 0" 1.0 1.0 0.0 0 0 0)
        (Default|CallOpentheDoor)))))

(fn ConstructionScript)

(fn UseKeyAutoGenFunc)